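; Cinderella enemy AI that behaves like a Weeping Angel, chasing the player unless it is being looked at.
; Each tick, a facing dot product and a visibility trace from the camera to the head socket decide whether it freezes movement and animation or resumes AI MoveTo.
; The first player overlap with its box triggers a jumpscare: a camera cut, sound and animation, then the view returns and a skeletal mesh starts simulating physics.
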(event `self.ReceiveTick`
  (params (DeltaSeconds :type "Float (single-precision)"))
  (bind _returnvalue (`GameplayStatics.GetPlayerCharacter` 0))
  ; Weeping Angel (Look = Stun)
  (if (> (`KismetMathLibrary.Dot_VectorVector` (`KismetMathLibrary.Normal` (- (`self.K2_GetActorLocation`) (`self.K2_GetActorLocation` _returnvalue))) (`self.GetActorForwardVector` _returnvalue)) 0.7)
    (bind (_outhit _returnvalue_2) (`KismetSystemLibrary.LineTraceSingle` :`Start` (`PlayerCameraManager.GetCameraLocation` (`GameplayStatics.GetPlayerCameraManager` 0)) :`End` (`SceneComponent.GetSocketLocation` (`self.Mesh`) "Head_Socket") :`TraceChannel` "TraceTypeQuery1" :`DrawDebugType` "ForOneFrame"))
    (if _returnvalue_2
      (set `SkeletalMeshComponent.GlobalAnimRateScale` 1.0 (`self.Mesh`) :!label _label)
      (`|AIMoveTo` self (0.0 0.0 0.0) (`GameplayStatics.GetPlayerCharacter` 0))
      (else
        (`MovementComponent.StopMovementImmediately` (`self.CharacterMovement`))
        (set `SkeletalMeshComponent.GlobalAnimRateScale` 0.0 (`self.Mesh`))))
    (else
      (goto _label))))

(event `self.Box.OnComponentBeginOverlap`
  (params (OverlappedComponent :type "PrimitiveComponent Object Reference") (OtherActor :type "Actor Object Reference") (OtherComp :type "PrimitiveComponent Object Reference") (OtherBodyIndex :type Integer) (bFromSweep :type Boolean) (SweepResult :type "HitResult Structure (by ref)"))
  ; Make Player Look At Angel When Attacked (For Dying Cutscene)
  (cast `/Game/a_Fairytale/Blueprints/BP_FirstPersonCharacter` OtherActor)
  (`/Engine/EditorBlueprintResources/StandardMacros.DoOnce` false
    (:`Completed`
      (`self.Jump Scare`))))

(event `Jump Scare`
  ; Make Player Look At Angel When Attacked (For Dying Cutscene)
  (`PlayerController.SetViewTargetWithBlend` (`GameplayStatics.GetPlayerController` 0) (`ActorComponent.GetOwner` (`self.Camera`)) 0.0 "VTBlend_Linear" 0.0 false)
  (`GameplayStatics.PlaySound2D` "/Game/a_Fairytale/Audio/SW_Flash.SW_Flash" 1.0 1.0 0.0 null null)
  (`SkeletalMeshComponent.PlayAnimation` (`self.SkeletalMesh`) "/Game/a_Fairytale/Characters/Anims/MF_Unarmed_Jog_Fwd.MF_Unarmed_Jog_Fwd" false)
  (`KismetSystemLibrary.Delay` 1.0)
  (`PlayerController.SetViewTargetWithBlend` (`GameplayStatics.GetPlayerController` 0) (`GameplayStatics.GetPlayerCharacter` 0) 0.0 "VTBlend_Linear" 0.0 false)
  (`GameplayStatics.GetActorOfClass` "/Game/a_Fairytale/Blueprints/BP_FirstPersonCharacter.BP_FirstPersonCharacter_C")
  (`PrimitiveComponent.SetSimulatePhysics` (`self.SkeletalMesh`) true))

(fn `UserConstructionScript`)