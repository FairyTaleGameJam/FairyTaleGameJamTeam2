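; Weeping-angel style enemy that chases the player and freezes while being watched.
; Each tick, a dot product tests whether the player faces it, then a visibility trace from the camera to its head socket checks for obstructions.
; When seen, it stops movement and pauses animation; otherwise it animates and calls AIMoveTo on the player.
; Player overlap with its box snaps the control rotation toward the angel.
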(event `self.ReceiveTick`
  (params (DeltaSeconds :type "Float (single-precision)"))
  (bind _returnvalue (`GameplayStatics.GetPlayerCharacter` 0))
  (if (> (`KismetMathLibrary.Dot_VectorVector` (`KismetMathLibrary.Normal` (- (`self.K2_GetActorLocation`) (`self.K2_GetActorLocation` _returnvalue))) (`self.GetActorForwardVector` _returnvalue)) 0.7)
    (bind (_outhit _returnvalue_2) (`KismetSystemLibrary.LineTraceSingle` :`Start` (`PlayerCameraManager.GetCameraLocation` (`GameplayStatics.GetPlayerCameraManager` 0)) :`End` (`SceneComponent.GetSocketLocation` (`self.Mesh`) "Head_Socket") :`TraceChannel` "TraceTypeQuery1" :`DrawDebugType` "ForOneFrame"))
    (if _returnvalue_2
      (set `SkeletalMeshComponent.GlobalAnimRateScale` 1.0 (`self.Mesh`) :!label _label)
      (`|AIMoveTo` self (0.0 0.0 0.0) (`GameplayStatics.GetPlayerCharacter` 0))
      (else
        (`MovementComponent.StopMovementImmediately` (`self.CharacterMovement`))
        (set `SkeletalMeshComponent.GlobalAnimRateScale` 0.0 (`self.Mesh`))))
    (else
      (goto _label))))

(event `self.Box.OnComponentBeginOverlap`
  (params (OverlappedComponent :type "PrimitiveComponent Object Reference") (OtherActor :type "Actor Object Reference") (OtherComp :type "PrimitiveComponent Object Reference") (OtherBodyIndex :type Integer) (bFromSweep :type Boolean) (SweepResult :type "HitResult Structure (by ref)"))
  (bind _returnvalue (`GameplayStatics.GetPlayerController` 0))
  (if (== OtherActor (`GameplayStatics.GetPlayerCharacter` 0))
    (`Controller.SetControlRotation` _returnvalue (`KismetMathLibrary.FindLookAtRotation` (`self.K2_GetActorLocation` _returnvalue) (`self.K2_GetActorLocation` self)))))

(fn `UserConstructionScript`)