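; Enemy AI character Blueprint that wanders at random until it spots a pawn, then chases and attacks the player.
; While unaware, Tick drives patrol-speed moves to random nearby reachable points after random delays.
; Pawn sensing sets a seen flag and triggers FollowPlayer, which moves to player 0 and plays a montage on arrival.
; A failed chase move or interrupted montage triggers another random wander move, and the seen flag never clears once set.
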(event `self.ReceiveTick`
  (params (DeltaSeconds :type "Float (single-precision)"))
  (if (not (`self.SeesPlayer`))
    (set `CharacterMovementComponent.MaxWalkSpeed` (`self.PatrolSpeed`) (`self.CharacterMovement`))
    (`KismetSystemLibrary.Delay` (`KismetMathLibrary.RandomFloatInRange` 2.0 5.0))
    (`|AIMoveTo` self (`NavigationSystemV1.K2_GetRandomReachablePointInRadius` (`self.K2_GetActorLocation`) 500.0 null null) null)))

(event `self.PawnSensing.OnSeePawn`
  (params (Pawn :type "Pawn Object Reference"))
  (set `self.SeesPlayer` true)
  (set `CharacterMovementComponent.MaxWalkSpeed` (`self.ChaseSpeed`) (`self.CharacterMovement`))
  (`self.FollowPlayer`))

(event `FollowPlayer`
  (set `self.CanAttack` true)
  (if (`self.SeesPlayer`)
    (`|AIMoveTo` self (0.0 0.0 0.0) (`GameplayStatics.GetPlayerCharacter` 0) 70.0
      (:`OnSuccess`
        (if (`self.CanAttack`)
          (set `self.CanAttack` false)
          (`|PlayMontage` null
            (:`then`
              (`KismetSystemLibrary.Delay` 0.2)
              (set `self.CanAttack` true))
            (:`OnInterrupted`
              (set `CharacterMovementComponent.MaxWalkSpeed` (`self.PatrolSpeed`) (`self.CharacterMovement`))
              (`KismetSystemLibrary.Delay` (`KismetMathLibrary.RandomFloatInRange` 2.0 5.0))
              (`|AIMoveTo` self (`NavigationSystemV1.K2_GetRandomReachablePointInRadius` (`self.K2_GetActorLocation`) 500.0 null null) null)))))
      (:`OnFail`
        (set `CharacterMovementComponent.MaxWalkSpeed` (`self.ChaseSpeed`) (`self.CharacterMovement`))
        (`KismetSystemLibrary.Delay` (`KismetMathLibrary.RandomFloatInRange` 2.0 5.0))
        (`|AIMoveTo` self (`NavigationSystemV1.K2_GetRandomReachablePointInRadius` (`self.K2_GetActorLocation`) 500.0 null null) null)))
    (else
      (set `self.SeesPlayer` false))))

(fn `UserConstructionScript`)